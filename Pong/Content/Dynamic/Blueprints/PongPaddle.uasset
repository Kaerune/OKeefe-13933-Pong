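; Pong actor that drives both paddles for two players on one keyboard and keeps the match score.
; Tick polls player controller 0 for W/S and Up/Down, moving the left and right paddle components with swept local X offsets scaled by PaddleSpeed and delta time.
; The AddScore event adds points to the chosen side's total and shows both scores via PrintString.
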(event Custom|AddScore
  (params (leftSide :type Boolean) (score :type Integer))
  (CallFunction|SetScore leftSide score score))

(event EventBeginPlay)

(event Collision|EventActorBeginOverlap
  (params (OtherActor :type Actor%20Object%20Reference)))

(event EventTick
  (params (DeltaSeconds :type Float%20%28single-precision%29))
  (Utilities|FlowControl|Sequence
    (:then_0
      (CallFunction|LeftPaddleUp DeltaSeconds))
    (:then_1
      (CallFunction|LeftPaddleDown DeltaSeconds))
    (:then_2
      (CallFunction|RightPaddleUp DeltaSeconds))
    (:then_3
      (CallFunction|RightPaddleDown DeltaSeconds))))

(fn ConstructionScript)

(fn LeftPaddleUp
  (params (A :type Float%20%28double-precision%29))
  (if (Game|Player|IsInputKeyDown (Game|GetPlayerController 0) "W")
    (Transformation|AddLocalOffset (Variables|Default|GetPaddle%20Left) (Math|Vector|MakeVector (* A (Variables|Default|GetpaddleSpeed)) 0.0 0.0) true false)))

(fn LeftPaddleDown
  (params (A :type Float%20%28double-precision%29))
  (if (Game|Player|IsInputKeyDown (Game|GetPlayerController 0) "S")
    (Transformation|AddLocalOffset (Variables|Default|GetPaddle%20Left) (Math|Vector|MakeVector (* A (Variables|Default|GetpaddleSpeed) -1.0) 0.0 0.0) true false)))

(fn RightPaddleUp
  (params (A :type Float%20%28double-precision%29))
  (if (Game|Player|IsInputKeyDown (Game|GetPlayerController 0) "Up")
    (Transformation|AddLocalOffset (Variables|Default|GetPaddle%20Right) (Math|Vector|MakeVector (* A (Variables|Default|GetpaddleSpeed)) 0.0 0.0) true false)))

(fn RightPaddleDown
  (params (A :type Float%20%28double-precision%29))
  (if (Game|Player|IsInputKeyDown (Game|GetPlayerController 0) "Down")
    (Transformation|AddLocalOffset (Variables|Default|GetPaddle%20Right) (Math|Vector|MakeVector (* A (Variables|Default|GetpaddleSpeed) -1.0) 0.0 0.0) true false)))

(fn SetScore
  (params (Condition :type Boolean) (B :type Integer) (B2 :type Integer))
  (if Condition
    (bind _output_get (Variables|Default|SetleftScore (+ (Variables|Default|GetleftScore) B2)))
    (else
      (bind _output_get_2 (Variables|Default|SetrightScore (+ (Variables|Default|GetrightScore) B)))))
  (Development|PrintString (Utilities|String|Append "Left: " (Utilities|String|ToString(Integer) _output_get) " 
" "Right: " (Utilities|String|ToString(Integer) _output_get_2))))