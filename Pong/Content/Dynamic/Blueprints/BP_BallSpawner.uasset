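; BP_BallSpawner is a spawner actor that creates balls and a BP_MultiBallSpawn actor at its own transform.
; BeginPlay spawns a ball at once and, after a delay, sets IsSpawnerSpawned, spawns BP_MultiBallSpawn, then prints a debug string after another delay.
; SpawnMultiBall and SpawnNewBall share the ball spawn node, whose class is unset here, with SpawnNewBall delaying first.
; The retry loop on IsSpawnerSpawned never repeats, since the flag is set true beforehand.
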(event Custom|SpawnNewBall
  (Utilities|FlowControl|Delay 2.0)
  (Game|SpawnActorfromClass "/Game/Dynamic/Blueprints/BP_PongBall.BP_PongBall_C" (Transformation|GetActorTransform) "Undefined" "MultiplyWithRoot" 0 0))

(event Custom|SpawnMultiBall
  (Game|SpawnActorfromClass "/Game/Dynamic/Blueprints/BP_PongBall.BP_PongBall_C" (Transformation|GetActorTransform) "Undefined" "MultiplyWithRoot" 0 0))

(event EventBeginPlay
  (Utilities|FlowControl|Sequence
    (:then_0
      (Game|SpawnActorfromClass "/Game/Dynamic/Blueprints/BP_PongBall.BP_PongBall_C" (Transformation|GetActorTransform) "Undefined" "MultiplyWithRoot" 0 0))
    (:then_1
      (Utilities|FlowControl|Delay 2.0)
      (Variables|Default|SetisSpawnerSpawned true)
      (Game|SpawnActorfromClass "/Game/Dynamic/Blueprints/BP_MultiBallSpawn.BP_MultiBallSpawn_C" (Transformation|GetActorTransform) "Undefined" "MultiplyWithRoot" 0 0 :!label _label)
      (Utilities|FlowControl|Delay 2.0)
      (if (Variables|Default|GetisSpawnerSpawned)
        (Development|PrintString "True")
        (else
          (goto _label))))))

(fn ConstructionScript)